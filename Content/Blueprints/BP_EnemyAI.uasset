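; Enemy AI Blueprint that patrols a set of placed point actors and prints a message when it sees a pawn.
; Point actor locations become a vector list walked with chained AI MoveTo calls, optionally looping or reversing the list to go back and forth.
; An InitializeEnemy event supplies route and options, restarting setup when patrolling.
; Flashlight components are destroyed when disabled, and Tick can draw a debug sight cone.
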(event OnSeePawn(PawnSensing)
  (params (Pawn :type Pawn%20Object%20Reference))
  (Development|PrintText "Player Spotted"))

(event Custom|ActivateFlashLight
  (bind _cylinder1 (Variables|Default|GetCylinder1))
  (bind _cylinder (Variables|Default|GetCylinder))
  (bind _spotlight (Variables|Default|GetSpotLight))
  (if (not (Variables|Default|GethasFlashlight))
    (Utilities|IsValid _spotlight
      (:Is%20Valid
        (Components|DestroyComponent _spotlight))
      (:Is%20Not%20Valid
        _))
    (Utilities|IsValid _cylinder
      (:Is%20Valid
        (Components|DestroyComponent _cylinder))
      (:Is%20Not%20Valid
        _))
    (Utilities|IsValid _cylinder1
      (:Is%20Valid
        (Components|DestroyComponent _cylinder1)))))

(event Custom|SetPositionVectors
  (for _array_element (Variables|Default|GetpositionActor)
    (Utilities|Array|Add (Variables|Default|GetpositionVectors) (Transformation|GetActorLocation _array_element))))

(event Custom|WalkToPoint
  (params (PointLocation :type Vector))
  (AI|AIMoveTo self PointLocation 0 5.0 false
    (:OnSuccess
      (Variables|Default|SetcurrentPoint (+ (Variables|Default|GetcurrentPoint) 1))
      (if (== (Variables|Default|GetcurrentPoint) (Utilities|Array|Length (Variables|Default|GetpositionVectors))) :!label _label
        (Variables|Default|SetcurrentPoint 0)
        (if (Variables|Default|GetpatrolsInLoop)
          (if (Variables|Default|GetpatrolBackandForth)
            (Utilities|Array|Reverse (Variables|Default|GetpositionVectors))
            (CallFunction|WalktoPoint (Utilities|Array|Get(acopy) (Variables|Default|GetpositionVectors) (Variables|Default|GetcurrentPoint)) :!label _label_2)
            (else
              (goto _label))))
        (else
          (goto _label_2))))))

(event Custom|PatrolingLoop
  (if (== (Variables|Default|GetcurrentPoint) (Utilities|Array|Length (Variables|Default|GetpositionVectors))) :!label _label
    (Variables|Default|SetcurrentPoint 0)
    (if (Variables|Default|GetpatrolsInLoop)
      (if (Variables|Default|GetpatrolBackandForth)
        (Utilities|Array|Reverse (Variables|Default|GetpositionVectors))
        (CallFunction|WalktoPoint (Utilities|Array|Get(acopy) (Variables|Default|GetpositionVectors) (Variables|Default|GetcurrentPoint)) :!label _label_2)
        (else
          (goto _label))))
    (else
      (goto _label_2))))

(event Custom|StartPatroling
  (CallFunction|SetPositionVectors)
  (CallFunction|PatrolingLoop))

(event Custom|InitializeEnemy
  (params (PositionActors :type Array%20of%20Actor%20Object%20References) (isPatrolling :type Boolean) (patrolBackAndForth :type Boolean) (patrolsInloop :type Boolean) (hasFlashFlight :type Boolean))
  (Variables|Default|SetpositionActor PositionActors)
  (Variables|Default|SethasFlashlight hasFlashFlight)
  (bind _output_get (Variables|Default|SetisPatrolling isPatrolling))
  (if _output_get
    (Variables|Default|SetpatrolsInLoop patrolsInloop)
    (Variables|Default|SetpatrolBackandForth patrolBackAndForth)
    (CallFunction|SetPositionVectors)
    (CallFunction|ActivateFlashLight)
    (CallFunction|PatrolingLoop)))

(event Collision|EventActorBeginOverlap
  (params (OtherActor :type Actor%20Object%20Reference)))

(event EventTick
  (params (DeltaSeconds :type Float%20%28single-precision%29))
  (bind _returnvalue (Transformation|GetActorTransform))
  (if (Variables|Default|GetdrawDebugSightCone)
    (Class|KismetSystemLibrary|DrawDebugConeinDegrees (+ (.location _returnvalue) "0.000000,0.000000,50.000000") (Math|Vector|GetForwardVector (.rotation _returnvalue)) 6.5e+02 18.0 18.0 12 "(R=0.044461,G=1.000000,B=0.000000,A=1.000000)" 0.0 0.0)))

(event EventBeginPlay
  (if (Variables|Default|GetisPatrolling)
    (CallFunction|SetPositionVectors)
    (CallFunction|ActivateFlashLight)
    (CallFunction|PatrolingLoop)
    (else
      (CallFunction|ActivateFlashLight))))

(fn ConstructionScript)